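; Demo player character for a networked shooter gun system, handling movement, aiming, cameras, HUD and weapon input.
; The server spawns gun and part inventories; switching sets CurrentWeapon, whose OnRep starts AnimBP swaps that call back to attach guns and update animations.
; Aiming and running apply locally and propagate via server RPCs, with aim multicast to other copies.
; Firing and reloading delegate to the gun; magazine hand-attachment moves only the mesh, avoiding desync.
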(event `self.ReceiveBeginPlay`
  (bind _startinggunpartsinventory (`self.StartingGunPartsInventory`))
  (bind _startinggunsinventory (`self.StartingGunsInventory`))
  (set `self.DemoAnimBp` (cast `/Game/ShooterGunSys/Animations/Character/AB_DemoCharacter` (`SkeletalMeshComponent.GetAnimInstance` (`self.Mesh`)) :!pure true)) ; Set a ref to our anim BP, so we \ndon't have to cast every time
  ;[1 1 1] Store the default value of the character's MaxWalkSpeed, so we can come back to it after we alter it (through running, aiming...)
  (set `self.DefaultMaxWalkSpeed` (`CharacterMovementComponent.MaxWalkSpeed` (`self.CharacterMovement`)))
  (if (`self.IsLocallyControlled`)
    (bind _returnvalue (`|CreateWidget` "/Game/ShooterGunSys/Blueprints/Widgets/HUD/WB_DemoHud.WB_DemoHud_C" (`self.DemoController`) self))
    (bind _output_get (set `self.Hud` _returnvalue))
    (`UserWidget.AddToViewport` _output_get 0))
  ;[1 1 1] This only gets executed on locally controlled characters in remote machines, because:
  ; 1) Non-locally controlled characters don't have a controller, so the cast will fail for them
  ; 2) Server locally controlled characters aren't yet possessed by their controllers at this point, so the cast will fail for them too
  (bind _asb_demo_controller (cast `/Game/ShooterGunSys/Blueprints/Controller/B_DemoController` (`self.GetController`))
    (:`then`
      (set `self.DemoController` _asb_demo_controller) ; Setting a reference to the \nDemoController here, since \nEventPossessed only happens \non the server copies, when \nremote copies aren't yet spawned
    )
    (:`CastFailed`
      _))
  (`/Engine/EditorBlueprintResources/ActorMacros.Switch Has Authority`
    (:`Authority`
      (bind _keys (`BlueprintMapLibrary.Map_Keys` _startinggunsinventory))
      (for _array_element _keys
        (for _ (range 1 (+ (`BlueprintMapLibrary.Map_Find` _startinggunsinventory _array_element) 1))
          (bind _returnvalue_2 (`|SpawnActorFromClass` :`Class` _array_element :`SpawnTransform` (`KismetMathLibrary.MakeTransform` (0.0 0.0 0.0)) :`CollisionHandlingOverride` "Undefined" :`TransformScaleMethod` "OverrideRootScale" :`Owner` self :`Instigator` null)) ; Spawn the guns indicated in the StartingInventory, with \ntheir default StartingParts
          (`self.K2_AttachToComponent` _returnvalue_2 (`self.Mesh`) "GunHolster" "SnapToTarget" "SnapToTarget" "KeepRelative" true)
          (`KismetArrayLibrary.Array_AddUnique` (`self.GunsInventory`) _returnvalue_2)))
      (set `self.CurrentWeapon` (`|GetArrayItem` (`self.GunsInventory`))) ; Set first gun
      (bind _keys_2 (`BlueprintMapLibrary.Map_Keys` _startinggunpartsinventory))
      (for _array_element_2 _keys_2
        (for _ (range 1 (+ (`BlueprintMapLibrary.Map_Find` _startinggunpartsinventory _array_element_2) 1))
          (bind _returnvalue_3 (`|SpawnActorFromClass` _array_element_2 (`KismetMathLibrary.MakeTransform` (0.0 0.0 200.0)) "AlwaysSpawn" "OverrideRootScale" self self))
          (`KismetArrayLibrary.Array_AddUnique` (`self.GunPartsInventory`) _returnvalue_3) ; Add to inventory
          (`self.SetActorHiddenInGame` _returnvalue_3 true))))))

(event `self.ReceivePossessed`
  (params (NewController :type "Controller Object Reference"))
  (set `self.DemoController` (cast `/Game/ShooterGunSys/Blueprints/Controller/B_DemoController` NewController :!pure true)) ; For the server local player, since \nat BeginPlay the server copies \naren't possessed yet
)

(event `InputAction|DeveloperTools`
  (params (Key :type "Key Structure"))
  ;[1 1 1] Show/hide the DeveloperTools widget on the HUD
  (:`Pressed`
    (`/Game/ShooterGunSys/Blueprints/Widgets/HUD/WB_DemoHud.ShowDeveloperTools` (`self.Hud`)))
  (:`Released`
    (`/Game/ShooterGunSys/Blueprints/Widgets/HUD/WB_DemoHud.HideDeveloperTools` (`self.Hud`))))

(event `InputAxis|Turn`
  (params (AxisValue :type "Float (single-precision)"))
  ;[1 1 1] Turn left and right. Store input amount to be used by the AnimBlueprint
  (`self.AddControllerYawInput` AxisValue)
  (set `self.InputAxisYaw` AxisValue))

(event `InputAxis|LookUp`
  (params (AxisValue :type "Float (single-precision)"))
  ;[1 1 1] Turn up and down. Store input amount to be used by the AnimBlueprint
  (`self.AddControllerPitchInput` AxisValue)
  (set `self.InputAxisPitch` AxisValue))

(event `InputAxis|MoveForward`
  (params (AxisValue :type "Float (single-precision)"))
  ;[1 1 1] Forward and backward stepping
  (`self.AddMovementInput` (`self.GetActorForwardVector`) AxisValue))

(event `InputAxis|MoveRight`
  (params (AxisValue :type "Float (single-precision)"))
  ;[1 1 1] Side stepping. Store input amount to be used by the AnimBlueprint
  (`self.AddMovementInput` (`self.GetActorRightVector`) AxisValue)
  (set `self.InputAxisRight` AxisValue))

(event `InputAction|Crouch`
  (params (Key :type "Key Structure"))
  ;[1 1 1] Using UE4's native Crouch and UnCrouch functions (natively replicated)
  (:`Pressed`
    (`self.Crouch`))
  (:`Released`
    (`self.UnCrouch`)))

(event `InputAction|Jump`
  (params (Key :type "Key Structure"))
  ;[1 1 1] Jump using UE4's native Jump and StopJumping functions (natively replicated)
  (:`Pressed`
    (`self.Jump`))
  (:`Released`
    (`self.StopJumping`)))

(event `self.K2_OnMovementModeChanged`
  (params (PrevMovementMode :type "EMovementMode Enum" :default "MOVE_None") (NewMovementMode :type "EMovementMode Enum" :default "MOVE_None") (PrevCustomMode :type Byte) (NewCustomMode :type Byte))
  ;[1 1 1] If we go into the air, exit aiming. EventOnMovementModeChanged is natively replicated by UE4
  (`/Engine/EditorBlueprintResources/StandardMacros.IsValid` (`self.DemoAnimBp`)
    (:`Is Valid`
      (if (and (`|EnumEquality` PrevMovementMode "MOVE_Walking") (`|EnumEquality` NewMovementMode "MOVE_Falling") (`self.IsAiming`))
        (`self.ExitAiming`)))))

(event `ServerRun`
  ;[1 1 1] Upon pressing the run button, exit aiming down sights, change MaxWalkSpeed locally and tell the server to change his MaxWalkSpeed too. MaxWalkSpeed is natively replicated, so when the server changes its value, it's replicated back to our local copy again (and all the other remote copies too)
  (set `self.IsRunPressed` true :!label _label)
  (set `CharacterMovementComponent.MaxWalkSpeed` (`self.RunSpeed`) (`self.CharacterMovement`)))

(event `InputAction|Run`
  (params (Key :type "Key Structure"))
  ;[1 1 1] Upon pressing the run button, exit aiming down sights, change MaxWalkSpeed locally and tell the server to change his MaxWalkSpeed too. MaxWalkSpeed is natively replicated, so when the server changes its value, it's replicated back to our local copy again (and all the other remote copies too)
  (:`Pressed`
    (if (`self.IsAiming`)
      (`self.ExitAiming`))
    (`self.ServerRun`)
    (goto _label))
  (:`Released`
    (`self.ServerStopRunning`)
    (set `self.IsRunPressed` false :!label _label_2)
    (set `CharacterMovementComponent.MaxWalkSpeed` (`self.DefaultMaxWalkSpeed`) (`self.CharacterMovement`))))

(event `ServerStopRunning`
  ;[1 1 1] Upon pressing the run button, exit aiming down sights, change MaxWalkSpeed locally and tell the server to change his MaxWalkSpeed too. MaxWalkSpeed is natively replicated, so when the server changes its value, it's replicated back to our local copy again (and all the other remote copies too)
  (goto _label_2))

(event `InputAction|CycleCameras`
  (params (Key :type "Key Structure"))
  ;[1 1 1] Cycle cameras
  (:`Pressed`
    (if (`ActorComponent.IsActive` (`self.FpCamera`))
      (`ActorComponent.SetActive` (`self.FpCamera`) false false)
      (`/Game/ShooterGunSys/Blueprints/Widgets/HUD/WB_DemoHud.UnhideCrosshair` (`self.Hud`)) ; Always show the crosshair when \nnot in 1P view
      (`ActorComponent.SetActive` (`self.TpCamera`) true false)
      (elif (`ActorComponent.IsActive` (`self.TpCamera`))
        (`ActorComponent.SetActive` (`self.TpCamera`) false false)
        (`ActorComponent.SetActive` (`self.DebugCameraA`) true false)
        (elif (`ActorComponent.IsActive` (`self.DebugCameraA`))
          (`ActorComponent.SetActive` (`self.DebugCameraA`) false false)
          (`ActorComponent.SetActive` (`self.DebugCameraB`) true false)
          (elif (`ActorComponent.IsActive` (`self.DebugCameraB`))
            (`ActorComponent.SetActive` (`self.DebugCameraB`) false false)
            (`ActorComponent.SetActive` (`self.DebugCameraC`) true false)
            (elif (`ActorComponent.IsActive` (`self.DebugCameraC`))
              (`ActorComponent.SetActive` (`self.DebugCameraC`) false false)
              (if (`self.IsAiming`)
                (`/Game/ShooterGunSys/Blueprints/Widgets/HUD/WB_DemoHud.HideCrosshair` (`self.Hud`)))
              (`ActorComponent.SetActive` (`self.FpCamera`) true false))))))))

(event `InputAction|Fire`
  (params (Key :type "Key Structure"))
  (bind _currentweapon (`self.CurrentWeapon`))
  (bind _currentweapon_2 (`self.CurrentWeapon`))
  ;[1 1 1] Tell weapon to start firing when trigger is pressed and stop when trigger is released. Fire mechanism and replication are done in the B_GunBase blueprint
  (:`Pressed`
    (`/Engine/EditorBlueprintResources/StandardMacros.IsValid` _currentweapon_2
      (:`Is Valid`
        (`/Game/ShooterGunSys/Blueprints/Guns/B_GunParent.StartFire` _currentweapon_2))))
  (:`Released`
    (`/Engine/EditorBlueprintResources/StandardMacros.IsValid` _currentweapon
      (:`Is Valid`
        (`/Game/ShooterGunSys/Blueprints/Guns/B_GunParent.StopFire` _currentweapon)))))

(event `ClientHitmarker`
  ;[1 1 1] Called by the server only, by the projectile blueprint or the gun's line trace function, when they hit a Pawn. Sent to the owning client only, to display the hitmarker on the HUD locally. Only the owning client has the HUD widget
  (`/Game/ShooterGunSys/Blueprints/Widgets/HUD/WB_DemoHud.HudHitmarker` (`self.Hud`)))

(event `InputAction|SwitchFireMode`
  (params (Key :type "Key Structure"))
  ;[1 1 1] Tell weapon to switch fire mode. Only needs to run locally
  (:`Pressed`
    (`/Game/ShooterGunSys/Blueprints/Guns/B_GunParent.SwitchFireMode` (`self.CurrentWeapon`))))

(event `self.ReceiveTick`
  (params (DeltaSeconds :type "Float (single-precision)"))
  (bind _returnvalue (`self.GetControlRotation`))
  (`/Engine/EditorBlueprintResources/ActorMacros.Switch Has Authority`
    (:`Authority`
      (bind _output_get (set `/Game/ShooterGunSys/Animations/Character/AB_DemoCharacter.ControlRot` _returnvalue (`self.DemoAnimBp`)))
      (set `self.ServerControlRot` _output_get) ; Replicate the control rotation to \nremote characters
    )
    (:`Remote`
      (if (`self.IsLocallyControlled`)
        (set `/Game/ShooterGunSys/Animations/Character/AB_DemoCharacter.ControlRot` _returnvalue (`self.DemoAnimBp`))
        (else
          (set `/Game/ShooterGunSys/Animations/Character/AB_DemoCharacter.ControlRot` (`self.ServerControlRot`) (`self.DemoAnimBp`)) ; Non-authority non-local \ncharacters use the rotation \nreplicated from the server
        )))))

(event `InputAction|Reload`
  (params (Key :type "Key Structure"))
  ;[1 1 1] Tell weapon to reload. Replication is done on the B_GunBase blueprint
  (:`Pressed`
    (`/Game/ShooterGunSys/Blueprints/Guns/B_GunParent.StartReload` (`self.CurrentWeapon`))))

(event `RemoveMag`
  (bind _magazine (`/Game/ShooterGunSys/Blueprints/Guns/B_GunParent.Magazine` (`self.CurrentWeapon`)))
  ;[1 1 1] Called from the anim BP. Mag goes from the weapon to the character's hand. Mag actor doesn't get actually detached from the gun, because this is for local visuals only. Instead, the mag's mesh gets detached from it's own root and later re-attached. This avoids network de-sync, etc. while still being visible to everyone
  (`SceneComponent.K2_AttachToComponent` (`self.GetComponentByClass` _magazine "/Script/Engine.MeshComponent") (`self.Mesh`) "hand_l" "KeepWorld" "KeepWorld" "KeepRelative" true)
  (set `self.MagInHand` _magazine) ; Ref to this specific mag, to \navoid confusion when \ninterrupted by SwitchWeapon
)

(event `InsertMag`
  (bind _maginhand (`self.MagInHand`))
  ;[1 1 1] Mag goes back. Called from the anim BP
  (`/Engine/EditorBlueprintResources/StandardMacros.IsValid` _maginhand
    (:`Is Valid`
      (`SceneComponent.K2_AttachToComponent` (`self.GetComponentByClass` _maginhand "/Script/Engine.MeshComponent") (`Actor.RootComponent` _maginhand) "None" "SnapToTarget" "SnapToTarget" "KeepRelative" true)
      (set `self.MagInHand` null) ; Empty the ref again when \nit's not in our hand anymore
    )))

(event `InputAction|NextWeapon`
  (params (Key :type "Key Structure"))
  (:`Pressed`
    (`/Game/ShooterGunSys/Blueprints/Guns/B_GunParent.StopFire` (`self.CurrentWeapon`))
    (if (`self.IsAiming`)
      (`self.ExitAiming`))
    (`self.ServerNextWeapon`)))

(event `ServerNextWeapon`
  (bind _gunsinventory (`self.GunsInventory`))
  (bind _returnvalue (`KismetArrayLibrary.Array_Find` _gunsinventory (`self.CurrentWeapon`)))
  (if (> (`KismetArrayLibrary.Array_Length` (`self.GunsInventory`)) 1)
    (if (== (`KismetArrayLibrary.Array_LastIndex` _gunsinventory) _returnvalue)
      (set `self.CurrentWeapon` (`|GetArrayItem` (`self.GunsInventory`)))
      (else
        (set `self.CurrentWeapon` (`|GetArrayItem` (`self.GunsInventory`) (+ _returnvalue 1)))))))

(event `SwitchWeapon`
  (bind _currentweapon (`self.CurrentWeapon`))
  (bind _currentweapon_2 (`self.CurrentWeapon`))
  (`/Engine/EditorBlueprintResources/StandardMacros.IsValid` (`self.LastWeapon`)
    (:`Is Valid`
      (`/Engine/EditorBlueprintResources/ActorMacros.Switch Has Authority`
        (:`Authority`
          (`self.K2_AttachToComponent` (`self.LastWeapon`) (`self.Mesh`) "GunHolster" "SnapToTarget" "SnapToTarget" "KeepRelative" true))
        (:`Remote`
          _))
      (if (`self.IsLocallyControlled`)
        (if (`self.IsAiming`)
          (`self.ExitAiming`)))
      (`/Game/ShooterGunSys/Blueprints/Guns/B_GunParent.UnEquip` (`self.LastWeapon`)) ; Run the gun's own UnEquip \nfunction
    )
    (:`Is Not Valid`
      _))
  (`/Engine/EditorBlueprintResources/ActorMacros.Switch Has Authority`
    (:`Authority`
      (`self.K2_AttachToComponent` (`self.CurrentWeapon`) (`self.Mesh`) "Gun" "SnapToTarget" "SnapToTarget" "KeepRelative" true)
      (`/Game/ShooterGunSys/Blueprints/Guns/B_GunParent.CalcHandTransforms` (`self.CurrentWeapon`)))
    (:`Remote`
      _))
  (bind _asab_demo_character (cast `/Game/ShooterGunSys/Animations/Character/AB_DemoCharacter` (`SkeletalMeshComponent.GetAnimInstance` (`self.Mesh`))))
  (set `/Game/ShooterGunSys/Animations/Character/AB_DemoCharacter.StandingBs` (`/Game/ShooterGunSys/Blueprints/Guns/B_GunParent.StandingBs` _currentweapon) _asab_demo_character)
  (set `/Game/ShooterGunSys/Animations/Character/AB_DemoCharacter.CrouchedBs` (`/Game/ShooterGunSys/Blueprints/Guns/B_GunParent.CrouchedBs` _currentweapon) _asab_demo_character)
  (set `/Game/ShooterGunSys/Animations/Character/AB_DemoCharacter.UnEquipSequence` (`/Game/ShooterGunSys/Blueprints/Guns/B_GunParent.UnEquipSequence` _currentweapon) _asab_demo_character)
  (set `/Game/ShooterGunSys/Animations/Character/AB_DemoCharacter.EquipSequence` (`/Game/ShooterGunSys/Blueprints/Guns/B_GunParent.EquipSequence` _currentweapon) _asab_demo_character)
  (set `/Game/ShooterGunSys/Animations/Character/AB_DemoCharacter.FireMontage` (`/Game/ShooterGunSys/Blueprints/Guns/B_GunParent.FireMontage` _currentweapon) _asab_demo_character)
  (set `/Game/ShooterGunSys/Animations/Character/AB_DemoCharacter.JumpStartSequence` (`/Game/ShooterGunSys/Blueprints/Guns/B_GunParent.JumpStartSequence` _currentweapon) _asab_demo_character)
  (set `/Game/ShooterGunSys/Animations/Character/AB_DemoCharacter.JumpLoopSequence` (`/Game/ShooterGunSys/Blueprints/Guns/B_GunParent.JumpLoopSequence` _currentweapon) _asab_demo_character)
  (set `/Game/ShooterGunSys/Animations/Character/AB_DemoCharacter.JumpEndSequence` (`/Game/ShooterGunSys/Blueprints/Guns/B_GunParent.JumpEndSequence` _currentweapon) _asab_demo_character)
  (set `/Game/ShooterGunSys/Animations/Character/AB_DemoCharacter.TimeToAim` (`/Game/ShooterGunSys/Blueprints/Guns/B_GunParent.TimeToAim` _currentweapon) _asab_demo_character)
  (set `/Game/ShooterGunSys/Animations/Character/AB_DemoCharacter.TimeFromAim` (`/Game/ShooterGunSys/Blueprints/Guns/B_GunParent.TimeFromAim` _currentweapon) _asab_demo_character)
  (set `/Game/ShooterGunSys/Animations/Character/AB_DemoCharacter.CycleSightsSpeed` (`/Game/ShooterGunSys/Blueprints/Guns/B_GunParent.CycleSightsSpeed` _currentweapon) _asab_demo_character)
  (`/Game/ShooterGunSys/Blueprints/Guns/B_GunParent.Equip` _currentweapon_2) ; Run the gun's own Equip function
  (set `self.LastWeapon` _currentweapon_2))

(event `InputAction|PrevWeapon`
  (params (Key :type "Key Structure"))
  (:`Pressed`
    (`/Game/ShooterGunSys/Blueprints/Guns/B_GunParent.StopFire` (`self.CurrentWeapon`))
    (if (`self.IsAiming`)
      (`self.ExitAiming`))
    (`self.ServerPrevWeapon`)))

(event `ServerPrevWeapon`
  (bind _gunsinventory (`self.GunsInventory`))
  (bind _returnvalue (`KismetArrayLibrary.Array_Find` (`self.GunsInventory`) (`self.CurrentWeapon`)))
  (if (> (`KismetArrayLibrary.Array_Length` (`self.GunsInventory`)) 1)
    (if (== _returnvalue 0)
      (set `self.CurrentWeapon` (`|GetArrayItem` _gunsinventory (`KismetArrayLibrary.Array_LastIndex` _gunsinventory)))
      (else
        (set `self.CurrentWeapon` (`|GetArrayItem` (`self.GunsInventory`) (- _returnvalue 1)))))))

(event `InputAction|Aim`
  (params (Key :type "Key Structure"))
  (:`Pressed`
    (`/Engine/EditorBlueprintResources/StandardMacros.IsValid` (`self.CurrentWeapon`)
      (:`Is Valid`
        ;[1 1 1] If the gun's HandTransform is 0, this means there's no sight positions calculated...
        (if (== (`self.HandTransform`) (`KismetMathLibrary.MakeTransform` (0.0 0.0 0.0)))
          (`KismetSystemLibrary.PrintString` "Can't aim down sights, gun has no sight position values" true true (struct :`R` 1.0 :`G` 0.978938 :`A` 1.0))
          (else
            ;[1 1 1] Aiming input can be customized for two styles: "Hold aim button to keep aiming" or "Press aim button again to stop aiming". This is set by the Customization variable 'IsHoldToAim'
            (if (`self.IsHoldToAim`)
              (if (not (`self.IsAiming`))
                (`self.EnterAiming` :!label _label))
              (elif (`self.IsAiming`)
                (`self.ExitAiming`)
                (else
                  (goto _label)))))))))
  (:`Released`
    (`/Engine/EditorBlueprintResources/StandardMacros.IsValid` (`self.CurrentWeapon`)
      (:`Is Valid`
        (if (`self.IsHoldToAim`)
          (if (`self.IsAiming`)
            (`self.ExitAiming`)))))))

(event `EnterAiming`
  (bind _hud (`self.Hud`))
  (bind _demoanimbp (`self.DemoAnimBp`))
  (bind _returnvalue (`SkeletalMeshComponent.GetAnimInstance` (`self.Mesh`)))
  ;[1 1 1] Only the locally controlled character checks if it's possible to enter aiming (not runnnig, not in air and not playing Reload, Equip or UnEquip animations). If it's possible, he enters aiming and sends the RPC to his server copy. The server copy then multicasts the command to all copies to enter aiming, including the server one and the locally controlled one, but this last one will ignore the multicast due to the 'IsLocallyControlled' check
  (if (not (or (`self.IsRunPressed`) (`NavMovementComponent.IsFalling` (`self.CharacterMovement`)) (`AnimInstance.IsPlayingSlotAnimation` _returnvalue (`/Game/ShooterGunSys/Blueprints/Guns/B_GunParent.UnEquipSequence` (`self.CurrentWeapon`)) "DefaultSlot") (`AnimInstance.IsPlayingSlotAnimation` _returnvalue (`/Game/ShooterGunSys/Blueprints/Guns/B_GunParent.EquipSequence` (`self.CurrentWeapon`)) "DefaultSlot")))
    (`self.ServerEnterAiming`)
    ;[1 1 1] Only locally controlled copies
    (if (`ActorComponent.IsActive` (`self.FpCamera`))
      (`/Engine/EditorBlueprintResources/StandardMacros.IsValid` _hud
        (:`Is Valid`
          (`/Game/ShooterGunSys/Blueprints/Widgets/HUD/WB_DemoHud.HideCrosshair` _hud))
        (:`Is Not Valid`
          _)))
    (bind _output_get (set `self.IsAiming` true))
    (set `/Game/ShooterGunSys/Blueprints/Guns/B_GunParent.IsAiming` _output_get (`self.CurrentWeapon`))
    (`/Engine/EditorBlueprintResources/StandardMacros.IsValid` _demoanimbp :!label _label_2
      (:`Is Valid`
        (set `/Game/ShooterGunSys/Animations/Character/AB_DemoCharacter.IsAiming` (`self.IsAiming`) _demoanimbp)
        ;[1 1 1] Change walking speed when aiming down sights. MaxWalkSpeed is natively replicated by UE4 and the value on the server is authoritative
        (set `CharacterMovementComponent.MaxWalkSpeed` (`self.WalkAimingSpeed`) (`self.CharacterMovement`))))))

(event `ServerEnterAiming`
  ;[1 1 1] Only the locally controlled character checks if it's possible to enter aiming (not runnnig, not in air and not playing Reload, Equip or UnEquip animations). If it's possible, he enters aiming and sends the RPC to his server copy. The server copy then multicasts the command to all copies to enter aiming, including the server one and the locally controlled one, but this last one will ignore the multicast due to the 'IsLocallyControlled' check
  (`self.MulticastEnterAiming`))

(event `MulticastEnterAiming`
  ;[1 1 1] Only the locally controlled character checks if it's possible to enter aiming (not runnnig, not in air and not playing Reload, Equip or UnEquip animations). If it's possible, he enters aiming and sends the RPC to his server copy. The server copy then multicasts the command to all copies to enter aiming, including the server one and the locally controlled one, but this last one will ignore the multicast due to the 'IsLocallyControlled' check
  (if (not (`self.IsLocallyControlled`))
    (set `self.IsAiming` true) ; Only non-locally controlled copies
    (goto _label_2)))

(event `ServerExitAiming`
  ;[1 1 1] The locally controlled copy calls ExitAiming and sends the RPC to the server copy. The server copy then multicasts the command to all copies to exit aiming, including the server one and the locally controlled one, but this last one will ignore the multicast due to the 'IsLocallyControlled' check
  (`self.MulticastExitAiming`))

(event `MulticastExitAiming`
  (bind _currentweapon (`self.CurrentWeapon`))
  (bind _demoanimbp (`self.DemoAnimBp`))
  ;[1 1 1] The locally controlled copy calls ExitAiming and sends the RPC to the server copy. The server copy then multicasts the command to all copies to exit aiming, including the server one and the locally controlled one, but this last one will ignore the multicast due to the 'IsLocallyControlled' check
  (if (not (`self.IsLocallyControlled`))
    ;[1 1 1] Update the current weapon and the anim blueprint
    (bind _output_get (set `self.IsAiming` false :!label _label_3))
    (`/Engine/EditorBlueprintResources/StandardMacros.IsValid` _demoanimbp
      (:`Is Valid`
        (bind _output_get_2 (set `/Game/ShooterGunSys/Animations/Character/AB_DemoCharacter.IsAiming` _output_get _demoanimbp))
        (`/Engine/EditorBlueprintResources/StandardMacros.IsValid` _currentweapon
          (:`Is Valid`
            (set `/Game/ShooterGunSys/Blueprints/Guns/B_GunParent.IsAiming` _output_get_2 _currentweapon))
          (:`Is Not Valid`
            _))
        (set `CharacterMovementComponent.MaxWalkSpeed` (`self.DefaultMaxWalkSpeed`) (`self.CharacterMovement`)) ; Reset walk speed to normal
      ))))

(event `ExitAiming`
  (bind _hud (`self.Hud`))
  ;[1 1 1] The locally controlled copy calls ExitAiming and sends the RPC to the server copy. The server copy then multicasts the command to all copies to exit aiming, including the server one and the locally controlled one, but this last one will ignore the multicast due to the 'IsLocallyControlled' check
  (`self.ServerExitAiming`)
  (`/Engine/EditorBlueprintResources/StandardMacros.IsValid` _hud
    (:`Is Valid`
      (`/Game/ShooterGunSys/Blueprints/Widgets/HUD/WB_DemoHud.UnhideCrosshair` _hud)
      (goto _label_3))
    (:`Is Not Valid`
      (goto _label_3))))

(event `InputAction|CycleSights`
  (params (Key :type "Key Structure"))
  (:`Pressed`
    (`/Game/ShooterGunSys/Blueprints/Guns/B_GunParent.ServerCycleSights` (`self.CurrentWeapon`))))

(fn `CanEnterGunCustomization`
  (returns (CanEnter :type Boolean))
  (bind _hud (`self.Hud`))
  (`/Engine/EditorBlueprintResources/StandardMacros.IsValid` _hud
    (:`Is Valid`
      (return (and (`|EnumEquality` (`Widget.GetVisibility` (`/Game/ShooterGunSys/Blueprints/Widgets/HUD/WB_DemoHud.DeveloperTools` _hud)) "Hidden") (== (`self.GetCurrentMontage`) null) (not (`self.IsAiming`)) (`ActorComponent.IsActive` (`self.FpCamera`)))))))

(fn `OnRep_CurrentWeapon`
  (bind _asab_demo_character (cast `/Game/ShooterGunSys/Animations/Character/AB_DemoCharacter` (`SkeletalMeshComponent.GetAnimInstance` (`self.Mesh`))))
  (`/Game/ShooterGunSys/Animations/Character/AB_DemoCharacter.SwitchWeapon` _asab_demo_character) ; Start anims
)

(fn `OnRep_GunPartsInventory`
  (bind _democontroller (`self.DemoController`))
  (bind _gcwidget (`/Game/ShooterGunSys/Blueprints/Controller/B_DemoController.GcWidget` _democontroller))
  (if (`self.IsLocallyControlled`)
    (`/Engine/EditorBlueprintResources/StandardMacros.IsValid` _democontroller
      (:`Is Valid`
        (`/Engine/EditorBlueprintResources/StandardMacros.IsValid` _gcwidget
          (:`Is Valid`
            (`/Game/ShooterGunSys/Blueprints/Widgets/GunCustomization/WB_GunCustomization.GenerateButtonsForParts` _gcwidget)))))))

(fn `OnRep_HandTransform`
  (if (== (`self.HandTransform`) (`KismetMathLibrary.MakeTransform` (0.0 0.0 0.0)))
    (`self.ExitAiming`) ; The last available sight was inactivated \nwhile we were aiming, so we exit aiming \nand don't send the transform of 0 to the \nanim, otherwise it kinda looks bad for a \nmoment
    (else
      (bind _asab_demo_character (cast `/Game/ShooterGunSys/Animations/Character/AB_DemoCharacter` (`SkeletalMeshComponent.GetAnimInstance` (`self.Mesh`))))
      (`/Game/ShooterGunSys/Animations/Character/AB_DemoCharacter.NewHandTransform` _asab_demo_character (`self.InterpolateSight`) (`self.HandTransform`)) ; Send this HandTransform to the anim
    )))

(fn `UserConstructionScript`)