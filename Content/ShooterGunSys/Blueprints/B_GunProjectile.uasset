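; B_GunProjectile is a gun projectile that spawns an impact effect and destroys itself when it hits something.
; On BeginPlay it makes its sphere and the instigator's capsule ignore each other when moving, so it cannot collide with its shooter.
; It is not replicated but spawned independently on server and clients, so it checks IsServer rather than HasAuthority.
; Only the server calls the B_DemoCharacter instigator's ClientHitmarker for Pawn hits.
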(event `self.ReceiveBeginPlay`
  (bind _instigator (`self.Instigator`))
  ;[1 1 1] Set projectile and instigator to not collide with each other
  (`PrimitiveComponent.IgnoreActorWhenMoving` (`self.Sphere`) _instigator true)
  (`PrimitiveComponent.IgnoreActorWhenMoving` (`self.GetComponentByClass` _instigator "/Script/Engine.CapsuleComponent") self true))

(event `self.ReceiveHit`
  (params (MyComp :type "PrimitiveComponent Object Reference") (Other :type "Actor Object Reference") (OtherComp :type "PrimitiveComponent Object Reference") (bSelfMoved :type Boolean) (HitLocation :type "Vector Structure") (HitNormal :type "Vector Structure") (NormalImpulse :type "Vector Structure") (Hit :type "HitResult Structure (by ref)"))
  (`GameplayStatics.SpawnEmitterAtLocation` "/Game/ShooterGunSys/Particles/P_Impact.P_Impact" HitLocation (`KismetMathLibrary.Conv_VectorToRotator` HitNormal)) ; Spawn impact effect when colliding
  ;[1 1 1] If the projectile hit a Pawn, call the shooter's hitmarker function
  (if (`KismetSystemLibrary.IsServer`)
    (cast `Pawn` Other
      (:`then`
        (`/Game/ShooterGunSys/Blueprints/Character/B_DemoCharacter.ClientHitmarker` (cast `/Game/ShooterGunSys/Blueprints/Character/B_DemoCharacter` (`self.Instigator`) :!pure true)))
      (:`CastFailed`
        _)))
  (`self.K2_DestroyActor`))

(fn `UserConstructionScript`)