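; Demo player controller that toggles gun customization for the controlled B_DemoCharacter's current weapon.
; Entering, allowed only when the character permits it, creates the customization widget, calls a server-named event to add the gun customization component, and disables character input.
; It uses Game and UI input with cursor, click and mouse-over events, so the gun itself stays clickable.
; Exiting removes widget and component and restores game-only input.
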(event `InputAction|GunCustomization`
  (params (Key :type "Key Structure"))
  (bind _gcwidget (`self.GcWidget`))
  (:`Pressed`
    (`/Engine/EditorBlueprintResources/StandardMacros.IsValid` (`self.GcWidget`) ; Are we already already in gun \ncustomization?
      (:`Is Valid`
        (`/Game/ShooterGunSys/Blueprints/Widgets/GunCustomization/WB_GunCustomization.ExitWidget` _gcwidget)
        (`Widget.RemoveFromParent` _gcwidget)
        (set `self.GcWidget` null)
        (`self.ServerRemoveGcComponent`)
        (`self.ExitGunCustomization`))
      (:`Is Not Valid`
        (bind _democharacter (`self.GetDemoCharacter`))
        (if (`/Game/ShooterGunSys/Blueprints/Character/B_DemoCharacter.CanEnterGunCustomization` _democharacter)
          (bind _returnvalue (`|CreateWidget` "/Game/ShooterGunSys/Blueprints/Widgets/GunCustomization/WB_GunCustomization.WB_GunCustomization_C" self (`/Game/ShooterGunSys/Blueprints/Character/B_DemoCharacter.CurrentWeapon` _democharacter) _democharacter))
          (bind _output_get (set `self.GcWidget` _returnvalue))
          (`UserWidget.AddToViewport` _output_get 0)
          (`self.ServerCreateGcComponent`)
          (`self.DisableInput` _democharacter null)
          (`WidgetBlueprintLibrary.SetInputMode_GameAndUIEx` self null) ; Apparently, mode UI only won't allow us to \nclick on the gun, just on the UI...
          (set `self.bShowMouseCursor` true)
          (set `self.bEnableMouseOverEvents` true)
          (set `self.bEnableClickEvents` true))))))

(event `ServerCreateGcComponent`
  (bind _democharacter (`self.GetDemoCharacter`))
  (bind _returnvalue (`AddComponent|NODE_AddB_GunCustomizationComponent-0` :`Gun` (`/Game/ShooterGunSys/Blueprints/Character/B_DemoCharacter.CurrentWeapon` _democharacter) :`DemoCharacter` _democharacter))
  (set `self.GcComponent` _returnvalue))

(event `ServerRemoveGcComponent`
  (`/Game/ShooterGunSys/Blueprints/Controller/B_GunCustomizationComponent.ExitComponent` (`self.GcComponent`))
  (set `self.GcComponent` null) ; Empy the var again
)

(event `ExitGunCustomization`
  (bind _democharacter (`self.GetDemoCharacter`))
  (`self.EnableInput` _democharacter null)
  (`WidgetBlueprintLibrary.SetInputMode_GameOnly` self)
  (set `self.bShowMouseCursor` false)
  (set `self.bEnableMouseOverEvents` false)
  (set `self.bEnableClickEvents` false))

(fn `UserConstructionScript`)