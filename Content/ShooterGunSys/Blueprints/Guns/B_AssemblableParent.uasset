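; Base class for assemblable guns and gun parts, handling sockets, attachment markers and replicated per-part state.
; On BeginPlay the authority builds optic, front and rear aimpoint arrays from socket name prefixes.
; It spawns or destroys clickable-style marker meshes on Base sockets matching a Top socket's type, and gathers attached parts recursively.
; RepNotify variables apply customization materials and trigger a child-overridable custom action, toggled through ServerAction.
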(event `self.ReceiveBeginPlay`
  (`self.GenerateAimpoints`) ; Server
  (set `self.IsCustomActioned` (`self.IsCustomActioned`)) ; Executes the CustomAction event
)

(event `GenerateAimpoints`
  (bind _returnvalue (`self.GetComponentByClass` "/Script/Engine.MeshComponent"))
  ;[1 1 1] Generate the three possible arrays of Aimpoint structs (OpticAimpoints, FrontAimpoints and RearAimpoints) for this gun part, according to the aimpoint sockets found in it. Aimpoint structs belong to the gun part, while SightData structs belong to the gun. SightData structs will be set on the gun according to the Aimpoint structs available on the parts attached to that gun
  (`/Engine/EditorBlueprintResources/ActorMacros.Switch Has Authority`
    (:`Authority`
      (for _array_element (`SceneComponent.GetAllSocketNames` _returnvalue)
        ;;[1 1 1] Optic Aimpoints
        (if (`KismetStringLibrary.StartsWith` (`KismetStringLibrary.Conv_NameToString` _array_element) "Aimpoint_Optic_")
          (`KismetArrayLibrary.Array_AddUnique` (`self.OpticAimpoints`) (make `/Game/ShooterGunSys/Blueprints/Structs/Aimpoint` _array_element _returnvalue))
          (else
            ;;[1 1 1] Front Aimpoints
            (if (`KismetStringLibrary.StartsWith` (`KismetStringLibrary.Conv_NameToString` _array_element) "Aimpoint_Front_")
              (`KismetArrayLibrary.Array_AddUnique` (`self.FrontAimpoints`) (make `/Game/ShooterGunSys/Blueprints/Structs/Aimpoint` _array_element _returnvalue))
              (else
                ;;[1 1 1] Rear Aimpoints
                (if (`KismetStringLibrary.StartsWith` (`KismetStringLibrary.Conv_NameToString` _array_element) "Aimpoint_Rear_")
                  (`KismetArrayLibrary.Array_AddUnique` (`self.RearAimpoints`) (make `/Game/ShooterGunSys/Blueprints/Structs/Aimpoint` _array_element _returnvalue)))))))))))

(event `ApplyMaterial`
  (params (NewMaterial :type "MaterialInterface Object Reference"))
  (set `self.Material` NewMaterial))

(event `ServerAction`
  (`self.InvertActioned`))

(event `CustomAction`
  (params (IsCustomActioned :type Boolean)))

(fn `Add Markers`
  (params (TopSocket :type Name))
  (bind _returnvalue (`self.GetComponentByClass` "/Script/Engine.MeshComponent"))
  (for _array_element (`SceneComponent.GetAllSocketNames` _returnvalue)
    (if (`KismetStringLibrary.StartsWith` (`KismetStringLibrary.Conv_NameToString` _array_element) (`KismetStringLibrary.Concat_StrStr` "Base_" (`|GetArrayItem` (`KismetStringLibrary.ParseIntoArray` (`KismetStringLibrary.Conv_NameToString` (`local.TopSocket`)) "_") 1) "_"))
      (bind _returnvalue_2 (`AddComponent|NODE_AddStaticMeshComponent-4` :`bManualAttachment` true))
      (`KismetArrayLibrary.Array_AddUnique` (`ActorComponent.ComponentTags` _returnvalue_2) "Marker")
      (set `PrimitiveComponent.bGenerateOverlapEvents` false _returnvalue_2)
      (`StaticMeshComponent.SetStaticMesh` _returnvalue_2 "/Game/ShooterGunSys/Meshes/Guns/GunParts/SM_PointMarker.SM_PointMarker")
      (`PrimitiveComponent.SetCollisionProfileName` _returnvalue_2 "UI")
      (`PrimitiveComponent.SetCollisionEnabled` _returnvalue_2 "QueryOnly")
      (`SceneComponent.K2_AttachToComponent` _returnvalue_2 _returnvalue _array_element "SnapToTarget" "SnapToTarget" "KeepRelative" true)
      (`SceneComponent.SetRelativeScale3D` _returnvalue_2 (`self.MarkerSize`)) ; Customize the marker size for this \npart (or gun)
      (`PrimitiveComponent.SetCastShadow` _returnvalue_2 false))))

(fn `DestroyMarkers`
  (bind (_arrayindex _arrayelement) (`/Engine/EditorBlueprintResources/StandardMacros.ReverseForEachLoop` (`self.GetComponentsByTag` "/Script/Engine.StaticMeshComponent" "Marker"))
    (:`LoopBody`
      (`ActorComponent.K2_DestroyComponent` _arrayelement))))

(fn `GetAttachedInternalLoop`
  (params (Part :type "/Game/ShooterGunSys/Blueprints/Guns/B_AssemblableParent Object Reference") (Parts :type "Array of /Game/ShooterGunSys/Blueprints/Guns/GunParts/B_GunPartParent Object Reference"))
  (for _array_element (`self.GetAttachedActors` Part true)
    (bind _asb_gun_part_parent (cast `/Game/ShooterGunSys/Blueprints/Guns/GunParts/B_GunPartParent` _array_element))
    (`KismetArrayLibrary.Array_AddUnique` Parts _asb_gun_part_parent)
    (`self.GetAttachedInternalLoop` _asb_gun_part_parent Parts))
  (return))

(fn `GetAttachedPartsRecursevely`
  (returns (Parts :type "Array of /Game/ShooterGunSys/Blueprints/Guns/GunParts/B_GunPartParent Object Reference"))
  (locals (PartsArray :type "Array of /Game/ShooterGunSys/Blueprints/Guns/GunParts/B_GunPartParent Object Reference"))
  (`self.GetAttachedInternalLoop` self (`local.PartsArray`))
  (return (`local.PartsArray`)))

(fn `OnRep_IsCustomActioned`
  (`self.CustomAction` (`self.IsCustomActioned`)))

(fn `OnRep_Material`
  (`PrimitiveComponent.SetMaterial` (`self.GetComponentByClass` "/Script/Engine.MeshComponent") 0 (`self.Material`)))

(fn `UserConstructionScript`)