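; Blueprint interface through which the Jigsaw inventory system communicates with a character.
; It declares hooks for adding widgets to named content, requesting server data for a component, checking weapon ammo count and loading saved data.
; Further hooks cover pickup interaction and interact actors going out of range.
; GetAnimationInfo exposes active slot, lean, aim-down-sights and crouch state, and the file holds only default return values.
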(fn `AddJigWidgetToContent`
  (params (WidgetRef :type "UserWidget Object Reference") (ContentName :type Text))
  (returns (Result :type Boolean))
  (return false))

(fn `GetAnimationInfo`
  (returns (ActiveSlot :type "/Game/JigSInventory/Jigsaw/Data/PlayerSlots Enum") (Leaning :type "Float (double-precision)") (Ads :type Boolean) (Crouched :type Boolean))
  (return "NewEnumerator0" 0.0 false false))

(fn `JigCheckWeaponAmmoCount`
  (returns (Result :type Boolean))
  (return false))

(fn `OnInteractActorOverDistance`
  (params (ActorRef :type "Actor Object Reference"))
  (returns (Result :type Boolean))
  (return false))

(fn `OnLoadSavedDataRequested`
  (returns (Result :type Boolean))
  (return false))

(fn `OnPickupInteractExecuted`
  (params (PickupRef :type "Actor Object Reference"))
  (returns (Result :type Boolean))
  (return false))

(fn `RequestServerData`
  (params (TargetComp :type "/Game/JigSInventory/Jigsaw/Components/BP_JigMultiplayer Object Reference"))
  (returns (Result :type Boolean))
  (return false))