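; Blueprint interface for the JigSInventory "JigMP" component, declaring callbacks for inventory events.
; It covers items added to or removed from main containers, the inventory and pickup actors, plus equip, consume, drop request, container swap and chamber UID update.
; Events pass item info, UIDs, container names or actor references, and all but the drop request return a boolean, with no logic in the interface itself.
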(fn `JigMP_OnItemAddedToInventory`
  (params (Info :type "/Game/JigSInventory/Jigsaw/Data/RepItemInfo Structure") (ToContainer :type Name))
  (returns (Result :type Boolean))
  (return false))

(fn `JigMP_OnItemConsumed`
  (params (Info :type "/Game/JigSInventory/Jigsaw/Data/RepItemInfo Structure") (Amount :type Integer))
  (returns (Result :type Boolean))
  (return false))

(fn `JigMP_OnItemEquipped`
  (params (ActorRef :type "Actor Object Reference") (ToContainerName :type Name) (UID :type Integer) (Info :type "/Game/JigSInventory/Jigsaw/Data/RepItemInfo Structure"))
  (returns (Result :type Boolean))
  (return false))

(fn `JigMP_OnItemRemovedFromInventory`
  (params (Info :type "/Game/JigSInventory/Jigsaw/Data/RepItemInfo Structure") (ToContainer :type Name :default "None"))
  (returns (Result :type Boolean))
  (return false))

(fn `JigMP_OnMainContainerItemAdded`
  (params (ToContainerUID :type Integer) (ItemUID :type Integer) (ToContainerName :type Name) (ItemInfo :type "/Game/JigSInventory/Jigsaw/Data/RepItemInfo Structure") (FromMain :type Name))
  (returns (Result :type Boolean) (ActorRef :type "Actor Object Reference"))
  (return false null))

(fn `JigMP_OnMainContainerItemRemoved`
  (params (FromContainerUID :type Integer) (ItemUID :type Integer) (ContainerName :type Name))
  (returns (Result :type Boolean))
  (return false))

(fn `JigMP_OnPickupItemAdded`
  (params (Info :type "/Game/JigSInventory/Jigsaw/Data/RepItemInfo Structure") (ToActor :type "Actor Object Reference"))
  (returns (Result :type Boolean))
  (return false))

(fn `JigMP_OnPickupItemRemoved`
  (params (Info :type "/Game/JigSInventory/Jigsaw/Data/RepItemInfo Structure") (FromActor :type "Actor Object Reference"))
  (returns (Result :type Boolean))
  (return false))

(fn `JigMP_OnRequestDropItem`
  (params (ItemInfo :type "/Game/JigSInventory/Jigsaw/Data/RepItemInfo Structure") (ContainerName :type Name))
  (returns (ActorRef :type "Actor Object Reference"))
  (return null))

(fn `JigMP_OnTwoContainersSwap`
  (params (FromContainer :type Name) (ToContainer :type Name))
  (returns (Result :type Boolean))
  (return false))

(fn `JigMP_OnUpdateChamberUID`
  (params (NewUID :type Integer))
  (returns (Result :type Boolean))
  (return false))