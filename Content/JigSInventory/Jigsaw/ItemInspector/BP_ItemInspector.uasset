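; Inventory item inspector actor that renders an item and its weapon attachments into a render target through a show-only scene capture.
; Inspect data fetched via the game state sets the static or skeletal mesh, transform and FOV zoom limits.
; Rotation turns a spring arm, and attachments become socketed child actors on lighting channel 1.
; To save work, changes trigger single captures unless continuous capture is switched on.
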(event `self.ReceiveBeginPlay`
  ;[0.02604 0.02604 0.02604] Begin play
  (`ActorComponent.Deactivate` (`self.SceneCaptureComponent2D`))
  (set `SceneCaptureComponent2D.FOVAngle` (`self.InitialFOV`) (`self.SceneCaptureComponent2D`))
  (set `SceneCaptureComponent.MaxViewDistanceOverride` 1000.0 (`self.SceneCaptureComponent2D`)))

(event `self.ReceiveEndPlay`
  (params (EndPlayReason :type "EEndPlayReason Enum" :default "Destroyed"))
  ;[0.005208 0.005208 0.005208] End play
  (set `/Game/JigSInventory/Jigsaw/Widgets/JSI_Slot.InspectorWidget` null (`self.ItemToInspect`))
  (`KismetRenderingLibrary.ReleaseRenderTarget2D` (`self.RenderT`)))

(fn `GetInitValues`
  (returns (ReturnValue :type "Transform Structure") (FOVAngle :type "Float (double-precision)"))
  (bind _skeletalmesh (`self.SkeletalMesh`))
  (return (`SceneComponent.GetRelativeTransform` (select `bool` (`KismetSystemLibrary.IsValid` (`SkinnedMeshComponent.SkeletalMesh` _skeletalmesh)) :`false` (`self.StaticMesh`) :`true` _skeletalmesh :!type "SceneComponent Object Reference")) (`SceneCaptureComponent2D.FOVAngle` (`self.SceneCaptureComponent2D`))))

(fn `GetRenderTarget`
  (returns (RenderT :type "TextureRenderTarget2D Object Reference"))
  (return (`self.RenderT`)))

(fn `InstallAttachment`
  (params (AttachmentID :type Name))
  (bind (_found _socket _type _class) (message `/Game/JigSInventory/Jigsaw/ItemInspector/IT_ItemSnapCaptor.GetLocalAttachmentByID` (`GameplayStatics.GetGameState`) AttachmentID))
  (if _found
    (bind _returnvalue (select `/Game/JigSInventory/Jigsaw/Data/AttachmentType` _type :`NewEnumerator0` (`self.Sight`) :`NewEnumerator1` (`self.Muzzle`) :`NewEnumerator2` (`self.Mag`) :`NewEnumerator3` (`self.HG_Grip`) :`NewEnumerator4` (`self.PistolGrip`) :`NewEnumerator5` (`self.Stock`) :`NewEnumerator6` (`self.Tactical1`)))
    (`ChildActorComponent.SetChildActorClass` _returnvalue _class)
    (`SceneComponent.K2_AttachToComponent` _returnvalue (`self.SkeletalMesh`) _socket "SnapToTarget" "SnapToTarget" "KeepRelative" true)
    (bind _childactor (`ChildActorComponent.ChildActor` _returnvalue))
    (`KismetArrayLibrary.Array_Add` (`SceneCaptureComponent.ShowOnlyActors` (`self.SceneCaptureComponent2D`)) _childactor)
    (`|ExecutionSequence`
      (:`then_0`
        (if (not (`ActorComponent.IsActive` (`self.SceneCaptureComponent2D`)))
          (`SceneCaptureComponent2D.CaptureScene` (`self.SceneCaptureComponent2D`))))
      (:`then_1`
        (bind _comp (message `/Game/JigSInventory/Jigsaw/ItemInspector/IT_ItemSnapCaptor.InspectorGetPrimitiveComponent` (`GameplayStatics.GetGameState`) _childactor))
        (`/Engine/EditorBlueprintResources/StandardMacros.IsValid` _comp
          (:`Is Valid`
            (`PrimitiveComponent.SetLightingChannels` _comp false true false)))))))

(fn `InstallAttachments`
  (params (AttachmentID :type "Array of Name"))
  (`|ExecutionSequence`
    (:`then_0`
      (for _array_element AttachmentID
        (bind (_found _socket _type _class) (message `/Game/JigSInventory/Jigsaw/ItemInspector/IT_ItemSnapCaptor.GetLocalAttachmentByID` (`GameplayStatics.GetGameState`) _array_element))
        (if _found
          (bind _returnvalue (select `/Game/JigSInventory/Jigsaw/Data/AttachmentType` _type :`NewEnumerator0` (`self.Sight`) :`NewEnumerator1` (`self.Muzzle`) :`NewEnumerator2` (`self.Mag`) :`NewEnumerator3` (`self.HG_Grip`) :`NewEnumerator4` (`self.PistolGrip`) :`NewEnumerator5` (`self.Stock`) :`NewEnumerator6` (`self.Tactical1`)))
          (`ChildActorComponent.SetChildActorClass` _returnvalue _class)
          (`SceneComponent.K2_AttachToComponent` _returnvalue (`self.SkeletalMesh`) _socket "SnapToTarget" "SnapToTarget" "KeepRelative" true)
          (bind _childactor (`ChildActorComponent.ChildActor` _returnvalue))
          (`KismetArrayLibrary.Array_Add` (`SceneCaptureComponent.ShowOnlyActors` (`self.SceneCaptureComponent2D`)) _childactor)
          (bind _comp (message `/Game/JigSInventory/Jigsaw/ItemInspector/IT_ItemSnapCaptor.InspectorGetPrimitiveComponent` (`GameplayStatics.GetGameState`) _childactor))
          (`/Engine/EditorBlueprintResources/StandardMacros.IsValid` _comp
            (:`Is Valid`
              (`PrimitiveComponent.SetLightingChannels` _comp false true false)))))
      (if (not (`ActorComponent.IsActive` (`self.SceneCaptureComponent2D`)))
        (`SceneCaptureComponent2D.CaptureScene` (`self.SceneCaptureComponent2D`))))
    (:`then_1`
      (return))))

(fn `OnZoomIn`
  (bind _scenecapturecomponent2d (`self.SceneCaptureComponent2D`))
  (set `SceneCaptureComponent2D.FOVAngle` (`KismetMathLibrary.FClamp` (+ (`SceneCaptureComponent2D.FOVAngle` _scenecapturecomponent2d) -5.0) (`self.MaxZoomInFOV`) (`self.MaxZoomOutFOV`)) _scenecapturecomponent2d)
  (if (not (`ActorComponent.IsActive` _scenecapturecomponent2d))
    (`SceneCaptureComponent2D.CaptureScene` (`self.SceneCaptureComponent2D`))))

(fn `OnZoomOut`
  (bind _scenecapturecomponent2d (`self.SceneCaptureComponent2D`))
  (set `SceneCaptureComponent2D.FOVAngle` (`KismetMathLibrary.FClamp` (+ (`SceneCaptureComponent2D.FOVAngle` _scenecapturecomponent2d) 5.0) (`self.MaxZoomInFOV`) (`self.MaxZoomOutFOV`)) _scenecapturecomponent2d)
  (if (not (`ActorComponent.IsActive` _scenecapturecomponent2d))
    (`SceneCaptureComponent2D.CaptureScene` (`self.SceneCaptureComponent2D`))))

(fn `RemoveAttachment`
  (params (AttachmentID :type Name))
  (bind (_found _socket _type) (message `/Game/JigSInventory/Jigsaw/ItemInspector/IT_ItemSnapCaptor.GetLocalAttachmentByID` (`GameplayStatics.GetGameState`) AttachmentID))
  (if _found
    (bind _returnvalue (select `/Game/JigSInventory/Jigsaw/Data/AttachmentType` _type :`NewEnumerator0` (`self.Sight`) :`NewEnumerator1` (`self.Muzzle`) :`NewEnumerator2` (`self.Mag`) :`NewEnumerator3` (`self.HG_Grip`) :`NewEnumerator4` (`self.PistolGrip`) :`NewEnumerator5` (`self.Stock`) :`NewEnumerator6` (`self.Tactical1`)))
    (`KismetArrayLibrary.Array_RemoveItem` (`SceneCaptureComponent.ShowOnlyActors` (`self.SceneCaptureComponent2D`)) (`ChildActorComponent.ChildActor` _returnvalue))
    (`ChildActorComponent.SetChildActorClass` _returnvalue null)
    (if (not (`ActorComponent.IsActive` (`self.SceneCaptureComponent2D`)))
      (`SceneCaptureComponent2D.CaptureScene` (`self.SceneCaptureComponent2D`)))))

(fn `SetCaptorActiveState`
  (params (IsActive :type Boolean))
  (bind _scenecapturecomponent2d (`self.SceneCaptureComponent2D`))
  (`ActorComponent.SetActive` _scenecapturecomponent2d IsActive false)
  (set `SceneCaptureComponent.bCaptureEveryFrame` IsActive _scenecapturecomponent2d))

(fn `SetItemToInspect`
  (params (ItemRef :type "/Game/JigSInventory/Jigsaw/Widgets/JSI_Slot Object Reference"))
  (bind _staticmesh (`self.StaticMesh`))
  (bind _skeletalmesh (`self.SkeletalMesh`))
  (`|ExecutionSequence`
    (:`then_0`
      ;[1 1 1] Create the render target
      (bind _returnvalue (`KismetRenderingLibrary.CreateRenderTarget2D` 512 512))
      (bind _output_get (set `SceneCaptureComponent2D.TextureTarget` _returnvalue (`self.SceneCaptureComponent2D`)))
      (set `self.RenderT` _output_get))
    (:`then_1`
      ;[0.05208 0.05208 0.05208] Set the mesh to inspect
      (bind _output_get_2 (set `self.ItemToInspect` ItemRef))
      (`|ExecutionSequence`
        (:`then_0`
          (bind _itemid (`/Game/JigSInventory/Jigsaw/Widgets/JSI_Slot.GetItemID` _output_get_2))
          (bind _out_row (`self.M_GetInspectInfo` _itemid)
            (:`Row Found`
              (`|ExecutionSequence`
                (:`then_0`
                  (`StaticMeshComponent.SetStaticMesh` (`self.StaticMesh`) null)
                  (`SkinnedMeshComponent.SetSkinnedAssetAndUpdate` (`self.SkeletalMesh`) null false))
                (:`then_1`
                  (bind ((`SMMeshToInspect_19_E54F2F3A4A046804996AC8858434A9D1` _smmeshtoinspect) (`SKMeshToInspect_22_3993354C4BB7822874A4DF833CAB68EB` _skmeshtoinspect) (`InspectLoc_11_C919533D46B727685EFE3C9F971FCF59` _inspectloc) (`InspectRot_14_E485A5024B0ACC12EE97CF91A17DA9F1` _inspectrot)) (break `/Game/JigSInventory/Jigsaw/ItemInspector/S_ItemInspectInfo` _out_row))
                  (`/Engine/EditorBlueprintResources/StandardMacros.IsValid` _skmeshtoinspect
                    (:`Is Valid`
                      (`SkinnedMeshComponent.SetSkinnedAssetAndUpdate` _skeletalmesh _skmeshtoinspect false)
                      (`SceneComponent.K2_SetRelativeLocationAndRotation` _skeletalmesh _inspectloc _inspectrot false true))
                    (:`Is Not Valid`
                      (`StaticMeshComponent.SetStaticMesh` _staticmesh _smmeshtoinspect)
                      (bind (_itemid_2 _smmeshtoinspect_2 _skmeshtoinspect_2 _inspectloc_2 _inspectrot_2 _initialfov _mazoominfov _mazoomoutfov) (break `/Game/JigSInventory/Jigsaw/ItemInspector/S_ItemInspectInfo` _out_row))
                      (`SceneComponent.K2_SetRelativeLocationAndRotation` _staticmesh _inspectloc_2 _inspectrot_2 false true)))
                  (set `self.MaxZoomInFOV` _mazoominfov)
                  (set `self.MaxZoomOutFOV` _mazoomoutfov)
                  (set `SceneCaptureComponent2D.FOVAngle` _initialfov (`self.SceneCaptureComponent2D`)))))
            (:`RowNotFound`
              (`KismetSystemLibrary.PrintString` (`KismetTextLibrary.Conv_TextToString` (`|FormatText` "Could not find {ItemID} in DT_ItemInspector data table" _itemid)) true true (struct :`R` 1.0 :`A` 1.0) 5.0))))
        (:`then_1`
          (`SceneCaptureComponent2D.CaptureScene` (`self.SceneCaptureComponent2D`)))))))

(fn `SetMeshRotation`
  (params (XYRot :type "Vector2D Structure"))
  (`SceneComponent.K2_AddLocalRotation` (`self.SpringArm`) (`KismetMathLibrary.MakeRotator` 0.0 XYRot_Y (* XYRot_X -1.0)) false false))

(fn `UpdateLocAndRot`
  (params (NewLocation :type "Vector Structure") (NewRotation :type "Rotator Structure") (FOVAngle :type "Float (double-precision)"))
  (`SceneComponent.K2_SetRelativeLocationAndRotation` (`self.StaticMesh`) NewLocation NewRotation false true)
  (`SceneComponent.K2_SetRelativeLocationAndRotation` (`self.SkeletalMesh`) NewLocation NewRotation false true)
  (set `SceneCaptureComponent2D.FOVAngle` FOVAngle (`self.SceneCaptureComponent2D`))
  (`SceneCaptureComponent2D.CaptureScene` (`self.SceneCaptureComponent2D`)))

(fn `UserConstructionScript`
  (set `SceneCaptureComponent.ShowOnlyActors` (`|MakeArray` self :!type "Actor Object Reference") (`self.SceneCaptureComponent2D`)))