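; BP_ItemSnapCaptor renders inventory and action bar images of Jigsaw inventory items with a show-only SceneCapture2D.
; SetJigitem loads the item's static or skeletal mesh, transform and FOV from GameState snap info.
; GetSnap captures into render targets sized by slot dimensions (fixed for action bar), optionally cached per ItemID for sharing.
; UpdateAttachments temporarily sockets child-actor attachments for the capture, moving them to lighting channel 1 and widening FOV for muzzles.
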(event `self.ReceiveBeginPlay`
  (set `SceneCaptureComponent2D.FOVAngle` (`self.InitialFOV`) (`self.SceneCaptureComponent2D`))
  (set `SceneCaptureComponent.MaxViewDistanceOverride` 1000.0 (`self.SceneCaptureComponent2D`)))

(fn `CaptureFromTarget`
  (params (TextureTarget :type "TextureRenderTarget2D Object Reference"))
  (bind _scenecapturecomponent2d (`self.SceneCaptureComponent2D`))
  (set `SceneCaptureComponent2D.TextureTarget` TextureTarget (`self.SceneCaptureComponent2D`))
  (`SceneCaptureComponent2D.CaptureScene` _scenecapturecomponent2d)
  (set `SceneCaptureComponent2D.TextureTarget` null _scenecapturecomponent2d))

(fn `ClearAttachments`
  (bind _showonlyactors (`SceneCaptureComponent.ShowOnlyActors` (`self.SceneCaptureComponent2D`)))
  (`KismetArrayLibrary.Array_Clear` _showonlyactors)
  (`KismetArrayLibrary.Array_Add` _showonlyactors self)
  (for _array_element (`|MakeArray` (`self.Sight`) (`self.Muzzle`) (`self.Mag`) (`self.HG_Grip`) (`self.PistolGrip`) (`self.Stock`) (`self.Tactical1`))
    (`ChildActorComponent.SetChildActorClass` _array_element null)
    (`SceneComponent.K2_AttachToComponent` _array_element (`self.SkeletalMesh`) "None" "KeepRelative" "KeepRelative" "KeepRelative" true)))

(fn `GetDefaultDim`
  (params (Target :type "/Game/JigSInventory/Jigsaw/Widgets/JSI_Slot Object Reference"))
  (returns (SlotDimension :type "Vector2D Structure"))
  (bind _slotdimension (`/Game/JigSInventory/Jigsaw/Widgets/JSI_Slot.GetSlotDim` Target))
  (bind (_x _y) (`KismetMathLibrary.BreakVector2D` _slotdimension))
  (if (and (!= _x _y) (not (`self.IsActionbar` Target)))
    (bind _returnvalue (`|GetDataTableRow` (`/Game/JigSInventory/Jigsaw/Widgets/JSI_Slot.GetDT` Target) (`/Game/JigSInventory/Jigsaw/Widgets/JSI_Slot.GetItemID` Target))
      (:`then`
        (return (`.SlotDimension_19_F030B0224A638DF8046DFBA1A9F61992` (break `/Game/JigSInventory/Jigsaw/Data/FItemInfo` _returnvalue)))))
    (else
      (return _slotdimension))))

(fn `GetInitValues`
  (returns (ReturnValue :type "Transform Structure") (FOVAngle :type "Float (double-precision)"))
  (bind _skeletalmesh (`self.SkeletalMesh`))
  (return (`SceneComponent.GetRelativeTransform` (select `bool` (`KismetSystemLibrary.IsValid` (`SkinnedMeshComponent.SkeletalMesh` _skeletalmesh)) :`false` (`self.StaticMesh`) :`true` _skeletalmesh :!type "SceneComponent Object Reference")) (`SceneCaptureComponent2D.FOVAngle` (`self.SceneCaptureComponent2D`))))

(fn `GetSnap`
  (params (ShareRTarget :type Boolean))
  (returns (Output_Get :type "TextureRenderTarget2D Object Reference") (`FromShared?` :type Boolean))
  (locals (RenderTarg :type "TextureRenderTarget2D Object Reference") (SaveRTarget :type Boolean))
  (bind _itemtoinspect (`self.ItemToInspect`))
  (bind _scenecapturecomponent2d (`self.SceneCaptureComponent2D`))
  (bind (_x _y) (`KismetMathLibrary.BreakVector2D` (select `bool` (`self.IsActionbar` _itemtoinspect) :`false` (* (`self.GetDefaultDim` _itemtoinspect) 60.0) :`true` (128.0 128.0))))
  (if ShareRTarget
    (bind _output_get (set `local.RenderTarg` (`BlueprintMapLibrary.Map_Find` (`self.CreatedRenderTargets`) (`.ItemID_107_1737366145EEBA44086DB6ACE0E9C90F` (break `/Game/JigSInventory/Jigsaw/Data/FItemInfo` (`/Game/JigSInventory/Jigsaw/Widgets/JSI_Slot.ItemInfo` _itemtoinspect))))))
    (`/Engine/EditorBlueprintResources/StandardMacros.IsValid` _output_get
      (:`Is Valid`
        (return (`local.RenderTarg`) true))
      (:`Is Not Valid`
        (set `local.SaveRTarget` true))))
  (bind _returnvalue (`KismetRenderingLibrary.CreateRenderTarget2D` (`KismetMathLibrary.FTrunc` _x) (`KismetMathLibrary.FTrunc` _y)))
  (bind _output_get_2 (set `local.RenderTarg` _returnvalue))
  (set `SceneCaptureComponent2D.TextureTarget` _output_get_2 (`self.SceneCaptureComponent2D`))
  (`SceneCaptureComponent2D.CaptureScene` _scenecapturecomponent2d)
  (set `SceneCaptureComponent2D.TextureTarget` null _scenecapturecomponent2d)
  (`|ExecutionSequence`
    (:`then_0`
      (if (`local.SaveRTarget`)
        (`BlueprintMapLibrary.Map_Add` (`self.CreatedRenderTargets`) (`.ItemID_107_1737366145EEBA44086DB6ACE0E9C90F` (break `/Game/JigSInventory/Jigsaw/Data/FItemInfo` (`/Game/JigSInventory/Jigsaw/Widgets/JSI_Slot.ItemInfo` (`self.ItemToInspect`)))) (`local.RenderTarg`))))
    (:`then_1`
      (return (`local.RenderTarg`) false))))

(fn `GetSnapNoCapture`
  (params (Item :type "/Game/JigSInventory/Jigsaw/Widgets/JSI_Slot Object Reference") (ShareRTarget :type Boolean))
  (returns (Output_Get :type "TextureRenderTarget2D Object Reference") (`FromShared?` :type Boolean))
  (locals (RenderTarg :type "TextureRenderTarget2D Object Reference") (SaveRTarget :type Boolean))
  (bind (_x _y) (`KismetMathLibrary.BreakVector2D` (select `bool` (`self.IsActionbar` Item) :`false` (* (`self.GetDefaultDim` Item) 60.0) :`true` (128.0 128.0))))
  (if ShareRTarget
    (bind _output_get (set `local.RenderTarg` (`BlueprintMapLibrary.Map_Find` (`self.CreatedRenderTargets`) (`.ItemID_107_1737366145EEBA44086DB6ACE0E9C90F` (break `/Game/JigSInventory/Jigsaw/Data/FItemInfo` (`/Game/JigSInventory/Jigsaw/Widgets/JSI_Slot.ItemInfo` Item))))))
    (`/Engine/EditorBlueprintResources/StandardMacros.IsValid` _output_get
      (:`Is Valid`
        (return (`local.RenderTarg`) true))
      (:`Is Not Valid`
        (set `local.SaveRTarget` true))))
  (bind _returnvalue (`KismetRenderingLibrary.CreateRenderTarget2D` (`KismetMathLibrary.FTrunc` _x) (`KismetMathLibrary.FTrunc` _y)))
  (set `local.RenderTarg` _returnvalue)
  (`|ExecutionSequence`
    (:`then_0`
      (if (`local.SaveRTarget`)
        (`BlueprintMapLibrary.Map_Add` (`self.CreatedRenderTargets`) (`.ItemID_107_1737366145EEBA44086DB6ACE0E9C90F` (break `/Game/JigSInventory/Jigsaw/Data/FItemInfo` (`/Game/JigSInventory/Jigsaw/Widgets/JSI_Slot.ItemInfo` (`local.Item`)))) (`local.RenderTarg`))))
    (:`then_1`
      (return (`local.RenderTarg`) false))))

(fn `InstallAttachments`
  (params (Attachments :type "Array of Name (by ref)"))
  (for _array_element Attachments
    (bind (_found _socket _type _class) (message `/Game/JigSInventory/Jigsaw/ItemInspector/IT_ItemSnapCaptor.GetLocalAttachmentByID` (`GameplayStatics.GetGameState`) _array_element))
    (if _found
      (bind _returnvalue (select `/Game/JigSInventory/Jigsaw/Data/AttachmentType` _type :`NewEnumerator0` (`self.Sight`) :`NewEnumerator1` (`self.Muzzle`) :`NewEnumerator2` (`self.Mag`) :`NewEnumerator3` (`self.HG_Grip`) :`NewEnumerator4` (`self.PistolGrip`) :`NewEnumerator5` (`self.Stock`) :`NewEnumerator6` (`self.Tactical1`)))
      (`ChildActorComponent.SetChildActorClass` _returnvalue _class)
      (`SceneComponent.K2_AttachToComponent` _returnvalue (`self.SkeletalMesh`) _socket "SnapToTarget" "SnapToTarget" "KeepRelative" true)
      (bind _childactor (`ChildActorComponent.ChildActor` _returnvalue))
      (`KismetArrayLibrary.Array_Add` (`SceneCaptureComponent.ShowOnlyActors` (`self.SceneCaptureComponent2D`)) _childactor)
      (bind _comp (message `/Game/JigSInventory/Jigsaw/ItemInspector/IT_ItemSnapCaptor.InspectorGetPrimitiveComponent` (`GameplayStatics.GetGameState`) _childactor))
      (`/Engine/EditorBlueprintResources/StandardMacros.IsValid` _comp
        (:`Is Valid`
          (`PrimitiveComponent.SetLightingChannels` _comp false true false)))))
  (`/Engine/EditorBlueprintResources/StandardMacros.IsValid` (`ChildActorComponent.ChildActor` (`self.Muzzle`))
    (:`Is Valid`
      (bind _output_get (set `SceneCaptureComponent2D.FOVAngle` (+ (stale _output_get) (* (`KismetMathLibrary.VSizeXY` (`.BoxExtent` (`self.GetActorBounds` (`ChildActorComponent.ChildActor` (`self.Muzzle`)) false false))) 0.5)) (`self.SceneCaptureComponent2D`))))))

(fn `IsActionbar`
  (params (ItemRef :type "/Game/JigSInventory/Jigsaw/Widgets/JSI_Slot Object Reference"))
  (returns (Result :type Boolean))
  (return (`/Game/JigSInventory/Jigsaw/Widgets/JSIContainer.IsActionbar` (`/Game/JigSInventory/Jigsaw/Widgets/JSI_Slot.ContainerMother` ItemRef))))

(fn `IsLocked`
  (returns (`IsLocked?` :type Boolean))
  (return (`self.IsLocked?`)))

(fn `SetJigitem`
  (params (ItemRef :type "/Game/JigSInventory/Jigsaw/Widgets/JSI_Slot Object Reference"))
  (returns (Found :type Boolean) (ShareRenderTargetWithSimilarItems :type Boolean))
  (locals (IsActionBarItem :type Boolean :default false))
  (bind _isactionbaritem (`local.IsActionBarItem`))
  ;[0.05208 0.05208 0.05208] Set the mesh to inspect
  (bind _output_get (set `self.ItemToInspect` ItemRef))
  (set `local.IsActionBarItem` (`self.IsActionbar` _output_get))
  (`|ExecutionSequence`
    (:`then_0`
      (bind _outputpin (`self.M_GetSnapInfo` (`/Game/JigSInventory/Jigsaw/Widgets/JSI_Slot.GetItemID` _output_get))
        (:`true`
          (bind ((`SMMeshToInspect_19_E54F2F3A4A046804996AC8858434A9D1` _smmeshtoinspect) (`SKMeshToInspect_22_3993354C4BB7822874A4DF833CAB68EB` _skmeshtoinspect) (`InspectLoc_11_C919533D46B727685EFE3C9F971FCF59` _inspectloc) (`InspectRot_14_E485A5024B0ACC12EE97CF91A17DA9F1` _inspectrot) (`UseAsInventoryImage_34_12F1BB53493360613AC8989046260606` _useasinventoryimage) (`ShareRenderTargetWithSimilarItems_37_0B8BEAFF45B73C1D0F96CAB2BE367900` _sharerendertargetwithsimilaritems) (`ActionBarLoc_41_40B718194C33C9157CAE68BEA98AEE8E` _actionbarloc) (`ActionBarRot_49_07A6011F4606CAFB778D38AD053DC404` _actionbarrot)) (break `/Game/JigSInventory/Jigsaw/ItemInspector/S_ItemInspectInfo` _outputpin))
          (if _useasinventoryimage
            (`|ExecutionSequence`
              (:`then_0`
                (`StaticMeshComponent.SetStaticMesh` (`self.StaticMesh`) null)
                (`SkinnedMeshComponent.SetSkinnedAssetAndUpdate` (`self.SkeletalMesh`) null false)
                (`SceneComponent.K2_SetRelativeLocationAndRotation` (`self.SkeletalMesh`) (`KismetMathLibrary.SelectVector` _actionbarloc _inspectloc _isactionbaritem) (`KismetMathLibrary.SelectRotator` _actionbarrot _inspectrot _isactionbaritem) false true)
                (`SceneComponent.K2_SetRelativeLocationAndRotation` (`self.StaticMesh`) (`KismetMathLibrary.SelectVector` _actionbarloc _inspectloc _isactionbaritem) (`KismetMathLibrary.SelectRotator` _actionbarrot _inspectrot _isactionbaritem) false true))
              (:`then_1`
                (`/Engine/EditorBlueprintResources/StandardMacros.IsValid` _skmeshtoinspect
                  (:`Is Valid`
                    (`SkinnedMeshComponent.SetSkinnedAssetAndUpdate` (`self.SkeletalMesh`) _skmeshtoinspect false))
                  (:`Is Not Valid`
                    (`StaticMeshComponent.SetStaticMesh` (`self.StaticMesh`) _smmeshtoinspect)))
                (bind ((`InitialFOV_25_D1CBFBEF4502434A72C272A2F65E6EB9` _initialfov) (`ActionBarFOV_47_F278A4974118C3202BBB4BBA5D8AEF23` _actionbarfov)) (break `/Game/JigSInventory/Jigsaw/ItemInspector/S_ItemInspectInfo` _outputpin))
                (set `SceneCaptureComponent2D.FOVAngle` (`KismetMathLibrary.SelectFloat` _actionbarfov _initialfov (`local.IsActionBarItem`)) (`self.SceneCaptureComponent2D`))
                (return true _sharerendertargetwithsimilaritems)))
            (else
              (return false false))))
        (:`false`
          (return false false))))
    (:`then_1`
      (return false false))))

(fn `SetJigitem_Custom`
  (params (ItemRef :type "/Game/JigSInventory/Jigsaw/Widgets/JSI_Slot Object Reference") (Location :type "Vector Structure") (Rotation :type "Rotator Structure") (FOV :type "Float (double-precision)"))
  (returns (Found :type Boolean) (ShareRenderTargetWithSimilarItems :type Boolean))
  (locals (IsActionBarItem :type Boolean :default false))
  ;[0.05208 0.05208 0.05208] Set the mesh to inspect
  (bind _output_get (set `self.ItemToInspect` ItemRef))
  (`|ExecutionSequence`
    (:`then_0`
      (bind _outputpin (`self.M_GetSnapInfo` (`/Game/JigSInventory/Jigsaw/Widgets/JSI_Slot.GetItemID` _output_get))
        (:`true`
          (bind ((`SMMeshToInspect_19_E54F2F3A4A046804996AC8858434A9D1` _smmeshtoinspect) (`SKMeshToInspect_22_3993354C4BB7822874A4DF833CAB68EB` _skmeshtoinspect) (`UseAsInventoryImage_34_12F1BB53493360613AC8989046260606` _useasinventoryimage) (`ShareRenderTargetWithSimilarItems_37_0B8BEAFF45B73C1D0F96CAB2BE367900` _sharerendertargetwithsimilaritems)) (break `/Game/JigSInventory/Jigsaw/ItemInspector/S_ItemInspectInfo` _outputpin))
          (if _useasinventoryimage
            (`|ExecutionSequence`
              (:`then_0`
                (`self.ClearAttachments`)
                (`StaticMeshComponent.SetStaticMesh` (`self.StaticMesh`) null)
                (`SkinnedMeshComponent.SetSkinnedAssetAndUpdate` (`self.SkeletalMesh`) null false)
                (`SceneComponent.K2_SetRelativeLocationAndRotation` (`self.SkeletalMesh`) (`local.Location`) (`local.Rotation`) false true)
                (`SceneComponent.K2_SetRelativeLocationAndRotation` (`self.StaticMesh`) (`local.Location`) (`local.Rotation`) false true))
              (:`then_1`
                (`/Engine/EditorBlueprintResources/StandardMacros.IsValid` _skmeshtoinspect
                  (:`Is Valid`
                    (`SkinnedMeshComponent.SetSkinnedAssetAndUpdate` (`self.SkeletalMesh`) _skmeshtoinspect false))
                  (:`Is Not Valid`
                    (`StaticMeshComponent.SetStaticMesh` (`self.StaticMesh`) _smmeshtoinspect)))
                (set `SceneCaptureComponent2D.FOVAngle` (`local.FOV`) (`self.SceneCaptureComponent2D`))
                (return true _sharerendertargetwithsimilaritems)))
            (else
              (return false false))))
        (:`false`
          (return false false))))
    (:`then_1`
      (return false false))))

(fn `SetLocked`
  (params (`IsLocked?` :type Boolean))
  (set `self.IsLocked?` `IsLocked?`))

(fn `UpdateAttachments`
  (params (ItemRef :type "/Game/JigSInventory/Jigsaw/Widgets/JSI_Slot Object Reference") (TextureTarget :type "TextureRenderTarget2D Object Reference") (Attachments :type "Array of Name (by ref)"))
  (returns (Output_Get :type "TextureRenderTarget2D Object Reference"))
  (bind _scenecapturecomponent2d (`self.SceneCaptureComponent2D`))
  (`self.SetJigitem` ItemRef)
  (`self.ClearAttachments`)
  (`self.InstallAttachments` Attachments)
  (bind _output_get (set `SceneCaptureComponent2D.TextureTarget` TextureTarget _scenecapturecomponent2d))
  (`SceneCaptureComponent2D.CaptureScene` _scenecapturecomponent2d)
  (set `SceneCaptureComponent2D.TextureTarget` null _scenecapturecomponent2d)
  (`self.ClearAttachments`)
  (return _output_get))

(fn `UpdateSnap`
  (params (ItemRef :type "/Game/JigSInventory/Jigsaw/Widgets/JSI_Slot Object Reference") (TextureTarget :type "TextureRenderTarget2D Object Reference"))
  (returns (Output_Get :type "TextureRenderTarget2D Object Reference"))
  (bind _scenecapturecomponent2d (`self.SceneCaptureComponent2D`))
  (`self.SetJigitem` ItemRef)
  (bind _output_get (set `SceneCaptureComponent2D.TextureTarget` TextureTarget _scenecapturecomponent2d))
  (`SceneCaptureComponent2D.CaptureScene` _scenecapturecomponent2d)
  (set `SceneCaptureComponent2D.TextureTarget` null _scenecapturecomponent2d)
  (return _output_get))

(fn `UserConstructionScript`
  (set `SceneCaptureComponent.ShowOnlyActors` (`|MakeArray` self :!type "Actor Object Reference") (`self.SceneCaptureComponent2D`)))